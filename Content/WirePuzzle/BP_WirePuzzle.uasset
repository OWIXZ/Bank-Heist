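; Possessable wire puzzle in which the player clicks BP_MasterWire cables in index order to detach them.
; Box overlap toggles input, and clicks trace from the cursor to compare each wire's index with the expected one.
; Completing the sequence or making a mistake shows a widget, then repossesses the third-person character, with failure also reattaching all cables.
; Unpossessing resets the character, after a delay if unsolved.
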(event OnComponentBeginOverlap(Box)
  (params (OverlappedComponent :type Primitive%20Component%20Object%20Reference) (OtherActor :type Actor%20Object%20Reference) (OtherComp :type Primitive%20Component%20Object%20Reference) (OtherBodyIndex :type Integer) (bFromSweep :type Boolean) (SweepResult :type Hit%20Result%20Structure%20%28by%20ref%29))
  (Utilities|Casting|CastToBP_ThirdPersonCharacter OtherActor)
  (Input|EnableInput (Game|GetPlayerController 0))
  (Variables|Default|SetPickUp true))

(event OnComponentEndOverlap(Box)
  (params (OverlappedComponent :type Primitive%20Component%20Object%20Reference) (OtherActor :type Actor%20Object%20Reference) (OtherComp :type Primitive%20Component%20Object%20Reference) (OtherBodyIndex :type Integer))
  (Utilities|Casting|CastToBP_ThirdPersonCharacter OtherActor)
  (Input|DisableInput (Game|GetPlayerController 0))
  (Variables|Default|SetPickUp false))

(event Custom|Failed%20Exit
  (bind _returnvalue (Game|GetPlayerController 0))
  (Widget|RemovefromParent (stale Input|MouseEvents|LeftMouseButton _returnvalue_5))
  (bind _outactors (Actor|GetAllActorsOfClass "/Game/WirePuzzle/BP_MasterWire.BP_MasterWire_C"))
  (for _array_element _outactors
    (Variables|/Script/CableComponent.CableComponent|SetbAttachEnd (Variables|/Game/WirePuzzle/BP_MasterWire.BP_MasterWire_C|GetCable _array_element) true)
    (bind _returnvalue_2 (Actor|GetActorOfClass "/Game/ThirdPerson/Blueprints/BP_ThirdPersonCharacter.BP_ThirdPersonCharacter_C"))
    (Pawn|Possess _returnvalue _returnvalue_2)
    (Rendering|SetActorHiddenInGame _returnvalue_2 false)
    (Variables|/Script/Engine.PlayerController|SetbShowMouseCursor _returnvalue false)
    (Variables|Default|SetDoor 0.0)))

(event EventBeginPlay)

(event EventUnpossessed
  (params (OldController :type Controller%20Object%20Reference))
  (if (Variables|Default|GetWin)
    _
    (else
      (Utilities|FlowControl|Delay 1e+01)))
  (bind _returnvalue (Actor|GetActorOfClass "/Game/ThirdPerson/Blueprints/BP_ThirdPersonCharacter.BP_ThirdPersonCharacter_C"))
  (Default|Reset _returnvalue))

(event Input|MouseEvents|LeftMouseButton
  (params (Key :type Key%20Structure :default "None"))
  (bind _returnvalue (Game|GetPlayerController 0))
  (bind _returnvalue_2 (Game|GetPlayerController 0))
  (bind (_worldlocation _worlddirection) (Game|Player|ConvertMouseLocationToWorldSpace _returnvalue_2))
  (:Pressed
    (if (not (Variables|Default|GetWin))
      (bind _outhit (Collision|LineTraceByChannel _worldlocation (+ _worldlocation (* _worlddirection 1e+03)) "TraceTypeQuery1" false 0 "ForOneFrame"))
      (if (.bBlockingHit (Collision|BreakHitResult _outhit))
        (bind _asbp_master_wire (Utilities|Casting|CastToBP_MasterWire (.HitActor (Collision|BreakHitResult _outhit))))
        (Variables|/Script/CableComponent.CableComponent|SetbAttachEnd (Variables|/Game/WirePuzzle/BP_MasterWire.BP_MasterWire_C|GetCable _asbp_master_wire) false)
        (if (== (Variables|/Game/WirePuzzle/BP_MasterWire.BP_MasterWire_C|GetWireIndex _asbp_master_wire) (Variables|Default|GetIndex))
          (bind _output_get (Variables|Default|SetIndex (+ (Variables|Default|GetIndex) 1) :!label _label))
          (if (== _output_get 6)
            (bind _returnvalue_3 (UserInterface|CreateWidget "/Game/WirePuzzle/W_WireSucceed.W_WireSucceed_C"))
            (UserInterface|Viewport|AddtoViewport _returnvalue_3 0)
            (Utilities|FlowControl|Delay 1.5)
            (Widget|RemovefromParent _returnvalue_3)
            (bind _returnvalue_4 (Actor|GetActorOfClass "/Game/ThirdPerson/Blueprints/BP_ThirdPersonCharacter.BP_ThirdPersonCharacter_C"))
            (Pawn|Possess _returnvalue _returnvalue_4)
            (Variables|/Script/Engine.PlayerController|SetbShowMouseCursor _returnvalue false)
            (Variables|Default|SetWin true)
            (Rendering|SetActorHiddenInGame _returnvalue_4 false))
          (elif (== (Variables|/Game/WirePuzzle/BP_MasterWire.BP_MasterWire_C|GetWireIndex _asbp_master_wire) (Variables|Default|GetIndex))
            (goto _label)
            (elif (== (Variables|/Game/WirePuzzle/BP_MasterWire.BP_MasterWire_C|GetWireIndex _asbp_master_wire) (Variables|Default|GetIndex))
              (goto _label)
              (elif (== (Variables|/Game/WirePuzzle/BP_MasterWire.BP_MasterWire_C|GetWireIndex _asbp_master_wire) (Variables|Default|GetIndex))
                (goto _label)
                (elif (== (Variables|/Game/WirePuzzle/BP_MasterWire.BP_MasterWire_C|GetWireIndex _asbp_master_wire) (Variables|Default|GetIndex))
                  (goto _label)
                  (else
                    (Variables|Default|SetIndex 1)
                    (bind _returnvalue_5 (UserInterface|CreateWidget "/Game/WirePuzzle/W_WireFail.W_WireFail_C"))
                    (UserInterface|Viewport|AddtoViewport _returnvalue_5 0)
                    (Utilities|FlowControl|Delay 1.5)
                    (CallFunction|FailedExit)))))))))))

(fn ConstructionScript)